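; Enemy AI pawn that chases the player once PawnSensing detects a pawn and plays a punch montage on reaching them.
; OnSeePawn sets a seen flag and starts an AI move to the player, with the montage length timing the attack cooldown.
; A self-repeating Patrol event walks four indexed points with random pauses, but nothing here starts it.
; Tick halts movement whenever the player is unseen.
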(event `self.ReceiveTick`
  (params (DeltaSeconds :type "Float (single-precision)"))
  (if (not (`self.isSeeingPlayer`))
    (`MovementComponent.StopMovementImmediately` (`self.CharacterMovement`))))

(event `self.PawnSensing.OnSeePawn`
  (params (Pawn :type "Pawn Object Reference"))
  (set `self.isSeeingPlayer` true)
  (`self.Follow Player`))

(event `Follow Player`
  (set `self.CanAttack` true)
  (if (`self.isSeeingPlayer`)
    (`|AIMoveTo` self (0.0 0.0 0.0) (`GameplayStatics.GetPlayerCharacter` 0) 70.0
      (:`OnSuccess`
        (if (`self.CanAttack`)
          (set `self.CanAttack` false)
          (bind _returnvalue (`self.PlayAnimMontage` "/Game/Animations/Ai/AM_Punch.AM_Punch"))
          (`KismetSystemLibrary.Delay` _returnvalue)
          (set `self.CanAttack` true)
          (else
            (set `self.isSeeingPlayer` false)))))))

(event `Patrol`
  ;[1 0 0.1429] Patrol
  (set `CharacterMovementComponent.MaxWalkSpeed` 150.0 (`self.CharacterMovement`))
  (`|AIMoveTo` self (`|GetArrayItem` (`self.PatrolLocation`) (`self.Locations`)) null
    (:`OnSuccess`
      (`KismetSystemLibrary.Delay` (`KismetMathLibrary.RandomFloatInRange` 1.0 3.0))
      (`self.Patrol`)
      (`/Engine/EditorBlueprintResources/StandardMacros.IncrementInt` (`self.Locations`)
        (:`  `
          (if (== (`self.Locations`) 4)
            (set `self.Locations` 0)))))))

(fn `UserConstructionScript`)