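; Dialogue component that shows and advances data-table-driven conversations on screen each time its Interaction event fires.
; The first interaction creates the W_Dialogue widget from the current row's name, line and image, and later ones update that same widget.
; Each row supplies the next row name and table, chaining lines across tables.
; A row's end flag makes the following interaction remove the widget.
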(event `Event Interaction`
  (if (`self.End Dialogue`)
    (`Widget.RemoveFromParent` (`self.Dialogue Ref`))
    (set `self.End Dialogue` false)
    (set `self.Dialogue Ref` null)
    (else
      (`/Engine/EditorBlueprintResources/StandardMacros.IsValid` (`self.Dialogue Ref`)
        (:`Is Valid`
          (bind _returnvalue (`|GetDataTableRow` (`self.Data Tabe`) (`self.Row Name`))
            (:`then`
              (bind (_name _dialogue _emotion _sound _speaker _dialougeend _rowname _datatable _image) (break `/Game/Blueprints/S_Dialogue` _returnvalue))
              (`/Game/Blueprints/W_Dialogue.Update Dialogue` (`self.Dialogue Ref`) _name (`self.In Brush Color`) _dialogue _image)
              (set `self.Row Name` _rowname)
              (set `self.Data Tabe` _datatable)
              (set `self.End Dialogue` _dialougeend))))
        (:`Is Not Valid`
          (bind _returnvalue_2 (`|GetDataTableRow` (`self.Data Tabe`) (`self.Row Name`))
            (:`then`
              (bind (_name_2 _dialogue_2 _emotion_2 _sound_2 _speaker_2 _dialougeend_2 _rowname_2 _datatable_2 _image_2) (break `/Game/Blueprints/S_Dialogue` _returnvalue_2))
              (bind _returnvalue_3 (`|CreateWidget` "/Game/Blueprints/W_Dialogue.W_Dialogue_C" null _name_2 (`self.In Brush Color`) _dialogue_2 _image_2))
              (bind _output_get (set `self.Dialogue Ref` _returnvalue_3))
              (`UserWidget.AddToViewport` _output_get 0)
              (set `self.Row Name` _rowname_2)
              (set `self.Data Tabe` _datatable_2)
              (set `self.End Dialogue` _dialougeend_2))))))))