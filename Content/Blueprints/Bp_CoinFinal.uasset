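; Collectible coin actor that the player picks up by touching it.
; When the player character overlaps its collision component, it sets IsCollected, passes itself to CoinsCollected on Bp_GameStateBase, then destroys itself.
; A separate updatecoin event destroys the coin without flagging or reporting it.
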(event `self.collison.OnComponentBeginOverlap`
  (params (OverlappedComponent :type "PrimitiveComponent Object Reference") (OtherActor :type "Actor Object Reference") (OtherComp :type "PrimitiveComponent Object Reference") (OtherBodyIndex :type Integer) (bFromSweep :type Boolean) (SweepResult :type "HitResult Structure (by ref)"))
  ;[0.5295 1 0] Comment
  (if (== OtherActor (`GameplayStatics.GetPlayerCharacter` 0))
    (set `self.IsCollected?` true)
    (bind _asbp_game_state_base (cast `/Game/Blueprints/Bp_GameStateBase` (`GameplayStatics.GetGameState`)))
    (`/Game/Blueprints/Bp_GameStateBase.CoinsCollected` _asbp_game_state_base self)
    (`self.K2_DestroyActor`)))

(event `update coin`
  ;[1 1 1] Comment
  (`self.K2_DestroyActor`))

(fn `UserConstructionScript`)