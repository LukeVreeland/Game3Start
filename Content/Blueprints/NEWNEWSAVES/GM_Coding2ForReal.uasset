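; Game mode that manages per-level save games, using the current level name as the save slot.
; BeginPlay loads an existing SG_LevelSave and its collected coins, deletes the slot if the cast fails, or creates a new save object if none exists.
; CheckPoint stores the player transform and saves.
; The transform restore on load sits behind a hardcoded condition and never runs.
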(event `self.ReceiveBeginPlay`
  (`KismetSystemLibrary.PrintString` "Loaded into the Gm_Coidng2ForReal Game Mode" true true (struct :`R` 1.0 :`G` 0.035189 :`A` 1.0) 20.0)
  (bind _returnvalue (`GameplayStatics.GetCurrentLevelName` true))
  (bind _returnvalue_2 (`GameplayStatics.DoesSaveGameExist` _returnvalue))
  (if _returnvalue_2
    (bind _returnvalue_3 (`GameplayStatics.LoadGameFromSlot` _returnvalue))
    (bind _assg_level_save (cast `/Game/Blueprints/NEWNEWSAVES/SG_LevelSave` _returnvalue_3)
      (:`then`
        (bind _output_get (set `self.Level Save` _assg_level_save))
        (`/Game/Blueprints/NEWNEWSAVES/SG_LevelSave.loadCollectedCoins` _output_get)
        (if (not true)
          (`SceneComponent.K2_SetWorldTransform` (`Character.CapsuleComponent` (`GameplayStatics.GetPlayerCharacter` 0)) (`/Game/Blueprints/NEWNEWSAVES/SG_LevelSave.PlayerTransform` (`self.Level Save`)) false false)))
      (:`CastFailed`
        (`GameplayStatics.DeleteGameInSlot` _returnvalue)))
    (else
      (bind _returnvalue_4 (`GameplayStatics.CreateSaveGameObject` "/Game/Blueprints/NEWNEWSAVES/SG_LevelSave.SG_LevelSave_C"))
      (set `self.Level Save` _returnvalue_4))))

(event `SaveGame`
  (bind _returnvalue (`GameplayStatics.GetCurrentLevelName` true))
  (`GameplayStatics.SaveGameToSlot` (`self.Level Save`) _returnvalue)
  (if true
    (`KismetSystemLibrary.PrintString` "SavedLevel")
    (else
      (`KismetSystemLibrary.PrintString` "did not SavedLevel"))))

(fn `CheckPoint`
  (params (PlayerTransform :type "Transform Structure"))
  (set `/Game/Blueprints/NEWNEWSAVES/SG_LevelSave.PlayerTransform` PlayerTransform (`self.Level Save`))
  (`self.SaveGame`))

(fn `UserConstructionScript`)