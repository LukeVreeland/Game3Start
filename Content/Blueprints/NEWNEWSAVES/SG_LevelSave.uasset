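; SG_LevelSave is a level save asset with functions for restoring collected coins and opened doors.
; LoadCollectedCoins calls LoadCollectedState on each valid element of its loop, but the CollectedCoins array and its length check appear disconnected.
; LoadOpenDoors loops through OpenedDoors when it has entries and checks validity, but takes no action on the doors.
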(fn `loadCollectedCoins`
  (locals (NewLocalVar :type Integer))
  (if true
    (for _array_element _
      (`/Engine/EditorBlueprintResources/StandardMacros.IsValid` _array_element
        (:`Is Valid`
          (`self.Load Collected State` _array_element))))))

(fn `LoadOpenDoors`
  (bind _openeddoors (`self.OpenedDoors`))
  (if (> (`KismetArrayLibrary.Array_Length` _openeddoors) 0)
    (for _array_element _openeddoors
      (`/Engine/EditorBlueprintResources/StandardMacros.IsValid` _array_element))))