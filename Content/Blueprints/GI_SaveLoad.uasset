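; GI_SaveLoad is an unfinished save/load Blueprint with SaveGame and LoadGame events, each printing a start message and checking whether the SlotName save exists.
; SaveGame loads the existing slot or creates a save game object, but never uses the result or writes it to the slot.
; LoadGame stops after the existence check, with nothing wired to load or apply data.
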(event `SaveGame`
  (`KismetSystemLibrary.PrintString` "Starting Save Game")
  (bind _returnvalue (`GameplayStatics.DoesSaveGameExist` (`self.slot name`)))
  (if _returnvalue
    (`GameplayStatics.LoadGameFromSlot` (`self.slot name`))
    (else
      (`GameplayStatics.CreateSaveGameObject` null))))

(event `Load Game`
  (`KismetSystemLibrary.PrintString` "Starting Load Game")
  (bind _returnvalue (`GameplayStatics.DoesSaveGameExist` (`self.slot name`)))
  (if _returnvalue
    _))