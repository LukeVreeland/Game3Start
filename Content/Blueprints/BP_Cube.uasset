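; BP_Cube is an interactable box actor that tells the third-person character when it can be interacted with.
; BeginPlay caches the character, and the Fwd component's begin and end overlaps set its CanInteractBox flag without checking which actor overlapped.
; Tick only prints the character's forward/backward axis state as debug text; nothing here moves the box.
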(event `self.ReceiveBeginPlay`
  (bind _returnvalue (`GameplayStatics.GetActorOfClass` "/Game/ThirdPerson/Blueprints/BP_ThirdPersonCharacter.BP_ThirdPersonCharacter_C"))
  (set `self.CharacterRef` _returnvalue))

(event `self.ReceiveTick`
  (params (DeltaSeconds :type "Float (single-precision)"))
  (bind _foward_backward_axis (`/Game/ThirdPerson/Blueprints/BP_ThirdPersonCharacter.Foward/Backward Axis` (`self.CharacterRef`)))
  (if true
    (if true
      (`|ExecutionSequence`
        (:`then_0`
          (if (== _foward_backward_axis 0.0)
            (`KismetSystemLibrary.PrintString` "Player is not moving foward/ backwards" true true (struct :`R` 1.0 :`G` 0.099749 :`A` 1.0))
            (elif (>= _foward_backward_axis 0.1)
              (`KismetSystemLibrary.PrintString` "Player is moving foward" true true (struct :`G` 0.557249 :`B` 1.0 :`A` 1.0))
              (else
                (`KismetSystemLibrary.PrintString` "Player is moving Backwards" true true (struct :`R` 0.020501 :`G` 1.0 :`B` 0.066947 :`A` 1.0))))))))))

(event `self.Fwd.OnComponentBeginOverlap`
  (params (OverlappedComponent :type "PrimitiveComponent Object Reference") (OtherActor :type "Actor Object Reference") (OtherComp :type "PrimitiveComponent Object Reference") (OtherBodyIndex :type Integer) (bFromSweep :type Boolean) (SweepResult :type "HitResult Structure (by ref)"))
  (`KismetSystemLibrary.PrintString` "Can Interact")
  (set `/Game/ThirdPerson/Blueprints/BP_ThirdPersonCharacter.CanInteractBox?` true (`self.CharacterRef`)))

(event `self.Fwd.OnComponentEndOverlap`
  (params (OverlappedComponent :type "PrimitiveComponent Object Reference") (OtherActor :type "Actor Object Reference") (OtherComp :type "PrimitiveComponent Object Reference") (OtherBodyIndex :type Integer))
  (`KismetSystemLibrary.PrintString` "Can Interact" true true (struct :`R` 1.0 :`G` 0.173764 :`A` 1.0))
  (set `/Game/ThirdPerson/Blueprints/BP_ThirdPersonCharacter.CanInteractBox?` false (`self.CharacterRef`)))

(fn `UserConstructionScript`)