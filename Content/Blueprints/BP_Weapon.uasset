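; BP_Weapon is a randomized weapon actor that destroys itself two seconds after BeginPlay.
; Its construction script picks a random row from DT_WeaponsFinal and applies that row's mesh.
; A dynamic M_Weapon material instance is tinted by the row's element through ElementSelect.
; DamageSelect then rolls Damage between the row's base damage and double that value.
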(event `self.ReceiveBeginPlay`
  (`KismetSystemLibrary.Delay` 2.0)
  (`self.K2_DestroyActor`))

(fn `Damage Select`
  (params (`Base Damage` :type "Float (double-precision)"))
  (set `self.Damage` (`KismetMathLibrary.RandomFloatInRange` `Base Damage` (* `Base Damage` 2.0)))
  (return))

(fn `Element Select`
  (params (Element :type "/Game/Blueprints/E_DamageTypeFinal Enum" :default "NewEnumerator0"))
  (returns (color :type "LinearColor Structure"))
  (switch `/Game/Blueprints/E_DamageTypeFinal` Element
    (:`NewEnumerator0`
      (return (struct :`R` 0.255154 :`G` 1.0 :`B` 0.406183 :`A` 1.0)))
    (:`NewEnumerator1`
      (return (struct :`R` 1.0 :`B` 0.022203 :`A` 1.0)))
    (:`NewEnumerator2`
      (return (struct :`G` 0.749181 :`B` 1.0 :`A` 1.0)))
    (:`NewEnumerator3`
      (return (struct :`G` 1.0 :`B` 0.160573 :`A` 1.0)))))

(fn `UserConstructionScript`
  (bind _static_object (`self.Static Object`))
  (bind _returnvalue (`|GetDataTableRow` "/Game/Blueprints/DT_WeaponsFinal.DT_WeaponsFinal" (`KismetStringLibrary.Conv_StringToName` (`KismetStringLibrary.Conv_IntToString` (`KismetMathLibrary.RandomIntegerInRange` 1 4))))
    (:`then`
      (bind (_model _type _element _damage) (break `/Game/Blueprints/S_WeaponFinal` _returnvalue))
      (`StaticMeshComponent.SetStaticMesh` _static_object _model)
      (bind _returnvalue_2 (`PrimitiveComponent.CreateDynamicMaterialInstance` _static_object 0 "/Game/Materials/M_Weapon.M_Weapon" "None"))
      (bind _color (`self.Element Select` _element))
      (`MaterialInstanceDynamic.SetVectorParameterValue` _returnvalue_2 "Diffusion" _color)
      (`self.Damage Select` _damage))))