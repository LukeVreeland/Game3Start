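; BP_CameraDoor is a door actor that slides a Door component with timeline-driven location lerps.
; QuietOpen events move it without a camera change and set Closed when finished, though one lerps between identical zero vectors.
; OpenDoor only branches on Closed and does nothing.
; A disconnected chain would blend the camera to the door, open it, wait, then blend back to a supplied view target.
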(event `Quiet Open`
  (bind (_direction _newtrack_0) (`Timeline|Timeline_0` :!via `PlayFromStart`)
    (:`Update`
      (`SceneComponent.K2_SetRelativeLocation` (`self.Door`) (`KismetMathLibrary.VLerp` (0.0 0.0 150.0) (0.0 0.0 -130.0) _newtrack_0) false false))
    (:`Finished`
      (set `self.Closed` true))))

(event `OpenDoor`
  (params (NewViewTarget :type "Actor Object Reference"))
  (if (`self.Closed`)
    _))

(event `QuietOpen`
  (bind (_direction _newtrack_0) (`Timeline|Timeline_1`)
    (:`Update`
      (`SceneComponent.K2_SetRelativeLocation` (`self.Door`) (`KismetMathLibrary.VLerp` (0.0 0.0 0.0) (0.0 0.0 0.0) _newtrack_0) false false))
    (:`Finished`
      (set `self.Closed` true))))

(fn `UserConstructionScript`)